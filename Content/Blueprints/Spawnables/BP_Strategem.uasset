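; BP_Strategem is a thrown-style physics ball that marks a spot on the ground with a temporary beacon.
; On BeginPlay it caches its owner as the third-person character, though nothing here uses that reference.
; A hit on a mostly upward-facing surface stops physics so the ball sticks, then spawns BP_Beacon at the impact point after a short delay.
; Seconds later it destroys both beacon and ball.
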(event Collision|EventHit
  (params (MyComp :type Primitive%20Component%20Object%20Reference) (Other :type Actor%20Object%20Reference) (OtherComp :type Primitive%20Component%20Object%20Reference) (bSelfMoved :type Boolean) (HitLocation :type Vector :default "0, 0, 0") (HitNormal :type Vector :default "0, 0, 0") (NormalImpulse :type Vector :default "0, 0, 0") (Hit :type Hit%20Result%20Structure%20%28by%20ref%29))
  ;[0.15 0.15 0.15 0.5] If strategem hits ground = stick, after stick spawn beacon at the ball for 5 seconds and then destory both ball and beacon
  (if (>= (.z HitNormal) 0.75)
    (Physics|SetSimulatePhysics (Variables|Default|GetStrategem) false)
    (Utilities|FlowControl|Delay 0.2)
    (bind _returnvalue (Game|SpawnActorfromClass "/Game/Blueprints/Spawnables/BP_Beacon.BP_Beacon_C" (Math|Transform|MakeTransform HitLocation "0, 0, 0" "1.000000,1.000000,1.000000") "Undefined" "MultiplyWithRoot" 0 0))
    (Utilities|FlowControl|Delay 5.0)
    (Actor|DestroyActor _returnvalue)
    (Actor|DestroyActor)))

(event EventBeginPlay
  ;[0.15 0.15 0.15 0.5] Get a ref to Player
  (bind _asbp_third_person_character (Utilities|Casting|CastToBP_ThirdPersonCharacter (Components|GetOwner)))
  (Variables|Default|SetAs%20BP%20Third%20Person%20Character _asbp_third_person_character))

(fn ConstructionScript)