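; BP_Mines is a spawnable mine carrier that lands, scatters a batch of mines, then destroys itself.
; A hit on a mostly upward-facing surface stops the cube's physics simulation and, after a short delay, sets the Islanded flag.
; While flagged, Tick uses a Delay to pace spawning BP_Mine at LaunchPoint, launching each with an upward, randomly sideways velocity impulse until the count limit is reached.
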(event Collision|EventHit
  (params (MyComp :type Primitive%20Component%20Object%20Reference) (Other :type Actor%20Object%20Reference) (OtherComp :type Primitive%20Component%20Object%20Reference) (bSelfMoved :type Boolean) (HitLocation :type Vector :default "0, 0, 0") (HitNormal :type Vector :default "0, 0, 0") (NormalImpulse :type Vector :default "0, 0, 0") (Hit :type Hit%20Result%20Structure%20%28by%20ref%29))
  ;[0.15 0.15 0.15 0.5] After Mine carrier is spawned check for when it has hit the ground, when it hits ground it stops all movement.
  (if (>= (.z HitNormal) 0.75)
    (Physics|SetSimulatePhysics (Variables|Default|GetCube) false)
    (Utilities|FlowControl|Delay 1.0)
    (Variables|Default|SetIslanded? true)))

(event EventTick
  (params (DeltaSeconds :type Float%20%28single-precision%29))
  (bind _count (Variables|Default|GetCount))
  ;[0.15 0.15 0.15 0.5] When mine carrier lands begin throwing out mines until count is reached, then destroy carrier and stop spawning mines
  (if (Variables|Default|GetIslanded?)
    (Utilities|FlowControl|Delay 0.2)
    (bind _returnvalue (Game|SpawnActorfromClass "/Game/Blueprints/Spawnables/BP_Mine.BP_Mine_C" (Math|Transform|MakeTransform (Transformation|GetWorldLocation (Variables|Default|GetLaunchPoint)) "0, 0, 0" "1.000000,1.000000,1.000000") "AlwaysSpawn" "MultiplyWithRoot" 0 0))
    (Physics|AddImpulse (Variables|/Game/Blueprints/Spawnables/BP_Mine.BP_Mine_C|GetMine _returnvalue) (Math|Vector|MakeVector (Math|Random|RandomFloatinRange -3e+02 3e+02) (Math|Random|RandomFloatinRange -3e+02 3e+02) 5e+02) "None" true)
    (Math|Integer|IncrementInt _count
      (:%20%20
        (if (>= _count 25)
          (Variables|Default|SetIslanded? false)
          (Actor|DestroyActor))))))

(fn ConstructionScript)